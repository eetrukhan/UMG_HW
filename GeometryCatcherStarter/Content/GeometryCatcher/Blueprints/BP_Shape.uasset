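; BP_Shape is a falling collectible in GeometryCatcher that the player catches to score.
; Each tick it moves down along world Z at FallSpeed, scaled by delta time, with sweep enabled.
; Overlapping a BP_Player reports its ColorNum to GameManager's IncrementShapesCollected, then destroys the shape.
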(event EventBeginPlay)

(event Collision|EventActorBeginOverlap
  (params (OtherActor :type Actor%20Object%20Reference))
  ;[1 1 1] Collect shape, increment score
  (Utilities|Casting|CastToBP_Player OtherActor)
  (Default|IncrementShapesCollected (Variables|Default|GetGameManager) (Variables|Default|GetColorNum self))
  (Actor|DestroyActor))

(event EventTick
  (params (DeltaSeconds :type Float%20%28single-precision%29))
  (Transformation|AddActorWorldOffset (Math|Vector|MakeVector 0.0 0.0 (* (* DeltaSeconds (Variables|Default|GetFallSpeed)) -1.0)) true))

(fn ConstructionScript)